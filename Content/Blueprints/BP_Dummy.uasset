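; Target dummy character that takes hits and can be stealth-assassinated from behind.
; Tick turns the health bar and assassination prompt toward the camera; an overlap radius shows the prompt to the player.
; Damage plays a random hit montage and sound, launches it along the player's facing, and updates BPCPlayerStats, ragdolling on death.
; StealthBackAssasin plays the victim montage, triggers delayed ragdoll and death sound, and returns a reference transform for the assassin.
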(event OnComponentBeginOverlap(AssasinationRadius)
  (params (OverlappedComponent :type Primitive%20Component%20Object%20Reference) (OtherActor :type Actor%20Object%20Reference) (OtherComp :type Primitive%20Component%20Object%20Reference) (OtherBodyIndex :type Integer) (bFromSweep :type Boolean) (SweepResult :type Hit%20Result%20Structure%20%28by%20ref%29))
  ;[0.05127 0.05127 0.05127] Assasination Overlap
  (Utilities|Casting|CastToBP_ThirdPersonCharacter OtherActor)
  (Rendering|SetVisibility (Variables|Default|GetAssasinate%20Widget) true false))

(event OnComponentEndOverlap(AssasinationRadius)
  (params (OverlappedComponent :type Primitive%20Component%20Object%20Reference) (OtherActor :type Actor%20Object%20Reference) (OtherComp :type Primitive%20Component%20Object%20Reference) (OtherBodyIndex :type Integer))
  ;[0.05127 0.05127 0.05127] Assasination Overlap
  (Utilities|Casting|CastToBP_ThirdPersonCharacter OtherActor)
  (Rendering|SetVisibility (Variables|Default|GetAssasinate%20Widget) false false))

(event Custom|RagDoll
  ;[0.05127 0.05127 0.05127] RagDoll
  (Utilities|FlowControl|Sequence
    (:then_0
      (Utilities|FlowControl|Delay 2.5)
      (Physics|SetSimulatePhysics (Variables|Character|GetMesh) true))
    (:then_1
      (Utilities|FlowControl|Delay 1.6)
      (Audio|PlaySoundatLocation "/Game/Audio/Hits/Die1.Die1" (Transformation|GetActorLocation) "0, 0, 0" 1.0 1.0 0.0 "/Game/Audio/SA_Character.SA_Character" 0 0 0))))

(event Collision|EventActorBeginOverlap
  (params (OtherActor :type Actor%20Object%20Reference)))

(event EventTick
  (params (DeltaSeconds :type Float%20%28single-precision%29))
  ;[0.05127 0.05127 0.05127] Event Tick / Dummy Above Text ([E] & HealthBar)
  (Transformation|SetWorldRotation (Variables|Default|GetAssasinate%20Widget) (Math|Rotator|FindLookatRotation (Transformation|GetWorldLocation (Variables|Default|GetAssasinate%20Widget)) (Transformation|GetWorldLocation (Variables|/Script/Engine.PlayerCameraManager|GetTransformComponent (Game|GetPlayerCameraManager 0)))) false false))

(event Game|Damage|EventAnyDamage
  (params (Damage :type Float%20%28single-precision%29) (DamageType :type Damage%20Type%20Object%20Reference) (InstigatedBy :type Controller%20Object%20Reference) (DamageCauser :type Actor%20Object%20Reference))
  ;[0.05127 0.05127 0.05127] Take Damage
  (Animation|PlayAnimMontage (Utilities|Array|Get(acopy) (Variables|Default|GethitAnims) (Math|Random|RandomIntegerinRange 0 (- (Utilities|Array|Length (Variables|Default|GethitAnims)) 1))) 1.0 "None")
  (bind _asbp_third_person_character (Utilities|Casting|CastToBP_ThirdPersonCharacter (Game|GetPlayerCharacter 0)))
  (Character|LaunchCharacter (* (Math|Vector|GetForwardVector (Transformation|GetActorRotation _asbp_third_person_character)) 6e+02) false false)
  (Audio|PlaySoundatLocation "/Game/Audio/Hits/Die1.Die1" (Transformation|GetActorLocation) "0, 0, 0" 1.0 (Math|Random|RandomFloatinRange 0.75 1.25) 0.0 "/Game/Audio/SA_Character.SA_Character" 0 0 0)
  (bind _isdead (Default|DecreaseHealth (Variables|Default|GetBPC_PlayerStats) Damage))
  (if _isdead
    (Physics|SetSimulatePhysics (Variables|Character|GetMesh) true)
    (Audio|PlaySoundatLocation "/Game/Audio/Hits/Die1.Die1" (Transformation|GetActorLocation) "0, 0, 0" 1.0 1.0 0.0 "/Game/Audio/SA_Character.SA_Character" 0 0 0)
    (Rendering|SetVisibility (Variables|Default|GetHeathBarWidget) false false)))

(event EventBeginPlay
  (bind _aswb_dummy_health (Utilities|Casting|CastToWB_DummyHealth (UserInterface|GetWidget (Variables|Default|GetHeathBarWidget))))
  (Variables|Default|SetDummyUI _aswb_dummy_health))

(fn ConstructionScript)

(fn StealthBackAssasin
  (Animation|PlayAnimMontage "/Game/Characters/Darius_Nightblade/Animations/Assanation/Paired_Knife_Stealth_KidneyAndNeck_Vic_Montage.Paired_Knife_Stealth_KidneyAndNeck_Vic_Montage" 1.0 "None")
  (CallFunction|RagDoll)
  (Rendering|SetVisibility (Variables|Default|GetAssasinate%20Widget) false false)
  (return (Transformation|GetWorldLocation (Variables|Default|GetAssasinationREF)) (Transformation|GetActorRotation)))