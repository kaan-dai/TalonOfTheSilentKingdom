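; Actor component that holds health, stamina, XP and level for BP_ThirdPersonCharacter, and health for BP_Dummy.
; BeginPlay waits a tick, casts the owner to set IsPlayer, then fills the matching UI.
; Functions change stats and push them straight to widgets; decreases return true at zero or below, while increase functions update only the player HUD.
; Reaching MaxXP levels up, raising the threshold, discarding overflow XP and playing sounds.
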(event EventBeginPlay
  ;[1 1 1] To Wait One Frame
  (Utilities|FlowControl|DelayUntilNextTick)
  (bind _asbp_third_person_character (Utilities|Casting|CastToBP_ThirdPersonCharacter (Components|GetOwner))
    (:then
      (Variables|Default|SetDariusBP _asbp_third_person_character)
      (Variables|Default|SetisPlayer true)
      (Progress|SetPercent (Variables|/Game/UI/WB_HUD.WB_HUD_C|GetStaminaBar (Variables|/Game/ThirdPerson/Blueprints/BP_ThirdPersonCharacter.BP_ThirdPersonCharacter_C|GetHUDWidget (Variables|Default|GetDariusBP))) (/ (Variables|Stamina|GetCurrentStamina) (Variables|Stamina|GetMaxStamina))))
    (:CastFailed
      ;[1 1 1] Set to Dummy
      (bind _asbp_dummy (Utilities|Casting|CastToBP_Dummy (Components|GetOwner)))
      (Variables|Default|SetDummpyBp _asbp_dummy)
      (Variables|Default|SetisPlayer false)))
  ;[1 1 1] Change Stats Btw Player and Dummy
  (Progress|SetPercent (select (Variables|Default|GetisPlayer) (Variables|/Game/UI/WB_HUD.WB_HUD_C|GetHealthBar (Variables|/Game/ThirdPerson/Blueprints/BP_ThirdPersonCharacter.BP_ThirdPersonCharacter_C|GetHUDWidget (Variables|Default|GetDariusBP))) (Variables|/Game/UI/WB_DummyHealth.WB_DummyHealth_C|GetDummyHealthBar (Variables|/Game/Blueprints/BP_Dummy.BP_Dummy_C|GetDummyUI (Variables|Default|GetDummpyBp)))) (/ (Variables|Health|GetCurrentHealth) (Variables|Health|GetMaxHealth)))
  (Rendering|Components|TextRender|SetText (select (Variables|Default|GetisPlayer) (Variables|/Game/UI/WB_HUD.WB_HUD_C|GetHealthText (Variables|/Game/ThirdPerson/Blueprints/BP_ThirdPersonCharacter.BP_ThirdPersonCharacter_C|GetHUDWidget (Variables|Default|GetDariusBP))) (Variables|/Game/UI/WB_DummyHealth.WB_DummyHealth_C|GetDummyHealthText (Variables|/Game/Blueprints/BP_Dummy.BP_Dummy_C|GetDummyUI (Variables|Default|GetDummpyBp)))) (Utilities|Text|ToText(Float) (Variables|Health|GetCurrentHealth) "HalfToEven"))
  (if (Variables|Default|GetisPlayer)
    (Progress|SetPercent (Variables|/Game/UI/WB_HUD.WB_HUD_C|GetXPBar (Variables|/Game/ThirdPerson/Blueprints/BP_ThirdPersonCharacter.BP_ThirdPersonCharacter_C|GetHUDWidget (Variables|Default|GetDariusBP))) (/ (Variables|XP|GetXP) (Variables|XP|GetMaxXP)))
    (Rendering|Components|TextRender|SetText (Variables|/Game/UI/WB_HUD.WB_HUD_C|GetXPText (Variables|/Game/ThirdPerson/Blueprints/BP_ThirdPersonCharacter.BP_ThirdPersonCharacter_C|GetHUDWidget (Variables|Default|GetDariusBP))) (Utilities|Text|FormatText "{Current XP} / {Max XP}" (Variables|XP|GetXP) (Variables|XP|GetMaxXP)))
    (Rendering|Components|TextRender|SetText (Variables|/Game/UI/WB_HUD.WB_HUD_C|GetLevelText (Variables|/Game/ThirdPerson/Blueprints/BP_ThirdPersonCharacter.BP_ThirdPersonCharacter_C|GetHUDWidget (Variables|Default|GetDariusBP))) (Utilities|Text|FormatText "Level  {Level}" (Variables|XP|GetLevel)))))

(fn DecreaseHealth
  (params (damage :type Float%20%28double-precision%29))
  ;[1 1 1] To Protect Everytime Calling It
  (if (not (<= (Variables|Health|GetCurrentHealth) 0.0))
    (bind _output_get (Variables|Health|SetCurrentHealth (- (Variables|Health|GetCurrentHealth) damage)))
    (Progress|SetPercent (select (Variables|Default|GetisPlayer) (Variables|/Game/UI/WB_HUD.WB_HUD_C|GetHealthBar (Variables|/Game/ThirdPerson/Blueprints/BP_ThirdPersonCharacter.BP_ThirdPersonCharacter_C|GetHUDWidget (Variables|Default|GetDariusBP))) (Variables|/Game/UI/WB_DummyHealth.WB_DummyHealth_C|GetDummyHealthBar (Variables|/Game/Blueprints/BP_Dummy.BP_Dummy_C|GetDummyUI (Variables|Default|GetDummpyBp)))) (/ _output_get (Variables|Health|GetMaxHealth)))
    (Rendering|Components|TextRender|SetText (select (Variables|Default|GetisPlayer) (Variables|/Game/UI/WB_HUD.WB_HUD_C|GetHealthText (Variables|/Game/ThirdPerson/Blueprints/BP_ThirdPersonCharacter.BP_ThirdPersonCharacter_C|GetHUDWidget (Variables|Default|GetDariusBP))) (Variables|/Game/UI/WB_DummyHealth.WB_DummyHealth_C|GetDummyHealthText (Variables|/Game/Blueprints/BP_Dummy.BP_Dummy_C|GetDummyUI (Variables|Default|GetDummpyBp)))) (Utilities|Text|ToText(Float) (Variables|Health|GetCurrentHealth) "HalfToEven"))
    (if (<= (Variables|Health|GetCurrentHealth) 0.0)
      _
      (else
        (return false))))
  (return true))

(fn IncreaseMaxHealth
  (params (increaseHealthPoint :type Float%20%28double-precision%29))
  (bind _dariusbp (Variables|Default|GetDariusBP))
  (bind _hudwidget (Variables|/Game/ThirdPerson/Blueprints/BP_ThirdPersonCharacter.BP_ThirdPersonCharacter_C|GetHUDWidget _dariusbp))
  (Variables|Health|SetMaxHealth (+ (Variables|Health|GetMaxHealth) increaseHealthPoint))
  (Progress|SetPercent (Variables|/Game/UI/WB_HUD.WB_HUD_C|GetHealthBar _hudwidget) (/ (Variables|Health|GetCurrentHealth) (Variables|Health|GetMaxHealth)))
  (Rendering|Components|TextRender|SetText (Variables|/Game/UI/WB_HUD.WB_HUD_C|GetHealthText _hudwidget) (Utilities|Text|ToText(Float) (Variables|Health|GetCurrentHealth) "HalfToEven")))

(fn DecreaseStamina
  (params (staminaDecreasePiont :type Float%20%28double-precision%29))
  (if (not (<= (Variables|Stamina|GetCurrentStamina) 0.0))
    (Variables|Stamina|SetCurrentStamina (- (Variables|Stamina|GetCurrentStamina) staminaDecreasePiont))
    (Progress|SetPercent (Variables|/Game/UI/WB_HUD.WB_HUD_C|GetStaminaBar (Variables|/Game/ThirdPerson/Blueprints/BP_ThirdPersonCharacter.BP_ThirdPersonCharacter_C|GetHUDWidget (Variables|Default|GetDariusBP))) (/ (Variables|Stamina|GetCurrentStamina) (Variables|Stamina|GetMaxStamina)))
    (if (<= (Variables|Stamina|GetCurrentStamina) 0.0)
      _
      (else
        (return false))))
  (return true))

(fn IncreaseMaxStamina
  (params (StaminaDecreasePiont :type Float%20%28double-precision%29) (B :type Float%20%28double-precision%29))
  (Variables|Stamina|SetMaxStamina (+ (Variables|Stamina|GetMaxStamina) B))
  (Progress|SetPercent (Variables|/Game/UI/WB_HUD.WB_HUD_C|GetStaminaBar (Variables|/Game/ThirdPerson/Blueprints/BP_ThirdPersonCharacter.BP_ThirdPersonCharacter_C|GetHUDWidget (Variables|Default|GetDariusBP))) (/ (Variables|Stamina|GetCurrentStamina) (Variables|Stamina|GetMaxStamina))))

(fn IncreaseHealth
  (params (addedHealth :type Float%20%28double-precision%29))
  (bind _dariusbp (Variables|Default|GetDariusBP))
  (bind _hudwidget (Variables|/Game/ThirdPerson/Blueprints/BP_ThirdPersonCharacter.BP_ThirdPersonCharacter_C|GetHUDWidget _dariusbp))
  (Variables|Health|SetCurrentHealth (+ (Variables|Health|GetCurrentHealth) addedHealth))
  (if (> (Variables|Health|GetCurrentHealth) (Variables|Health|GetMaxHealth))
    (Variables|Health|SetCurrentHealth (Variables|Health|GetMaxHealth)))
  (Progress|SetPercent (Variables|/Game/UI/WB_HUD.WB_HUD_C|GetHealthBar _hudwidget) (/ (Variables|Health|GetCurrentHealth) (Variables|Health|GetMaxHealth)))
  (Rendering|Components|TextRender|SetText (Variables|/Game/UI/WB_HUD.WB_HUD_C|GetHealthText _hudwidget) (Utilities|Text|ToText(Float) (Variables|Health|GetCurrentHealth) "HalfToEven")))

(fn IncreaseStamina
  (params (addedStamina :type Float%20%28double-precision%29))
  (Variables|Stamina|SetCurrentStamina (+ (Variables|Stamina|GetCurrentStamina) addedStamina))
  (if (> (Variables|Stamina|GetCurrentStamina) (Variables|Stamina|GetMaxStamina))
    (Variables|Stamina|SetCurrentStamina (Variables|Stamina|GetMaxStamina)))
  (Progress|SetPercent (Variables|/Game/UI/WB_HUD.WB_HUD_C|GetStaminaBar (Variables|/Game/ThirdPerson/Blueprints/BP_ThirdPersonCharacter.BP_ThirdPersonCharacter_C|GetHUDWidget (Variables|Default|GetDariusBP))) (/ (Variables|Stamina|GetCurrentStamina) (Variables|Stamina|GetMaxStamina))))

(fn IncreaseXP
  (params (addedXPPoint :type Float%20%28double-precision%29))
  (Variables|XP|SetXP (+ (Variables|XP|GetXP) addedXPPoint))
  (if (>= (Variables|XP|GetXP) (Variables|XP|GetMaxXP))
    (XP|IncreaseLevel 1))
  (Progress|SetPercent (Variables|/Game/UI/WB_HUD.WB_HUD_C|GetXPBar (Variables|/Game/ThirdPerson/Blueprints/BP_ThirdPersonCharacter.BP_ThirdPersonCharacter_C|GetHUDWidget (Variables|Default|GetDariusBP))) (/ (Variables|XP|GetXP) (Variables|XP|GetMaxXP)))
  (Rendering|Components|TextRender|SetText (Variables|/Game/UI/WB_HUD.WB_HUD_C|GetXPText (Variables|/Game/ThirdPerson/Blueprints/BP_ThirdPersonCharacter.BP_ThirdPersonCharacter_C|GetHUDWidget (Variables|Default|GetDariusBP))) (Utilities|Text|FormatText "{Current XP} / {Max XP}" (Variables|XP|GetXP) (Variables|XP|GetMaxXP))))

(fn IncreaseLevel
  (params (addedLevel :type Integer))
  (Variables|XP|SetLevel (+ (Variables|XP|GetLevel) addedLevel))
  (Variables|XP|SetMaxXP (+ (Variables|XP|GetMaxXP) 1.5e+02))
  (Variables|XP|SetXP 0.0)
  (Rendering|Components|TextRender|SetText (Variables|/Game/UI/WB_HUD.WB_HUD_C|GetLevelText (Variables|/Game/ThirdPerson/Blueprints/BP_ThirdPersonCharacter.BP_ThirdPersonCharacter_C|GetHUDWidget (Variables|Default|GetDariusBP))) (Utilities|Text|FormatText "Level  {Level}" (Variables|XP|GetLevel)))
  (Audio|PlaySound2D "/Game/Audio/UI/Level.Level" 1.0 1.0 0.0 0 0)
  (Audio|PlaySound2D "/Game/Audio/UI/XP.XP" 2.0 1.0 0.0 0 0))