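; Actor component that gives BP_ThirdPersonCharacter a four-step melee combo of sword attacks and a kick.
; IA_Attack plays the montage for the current AttackIndex, while SwordAttackCombo continues saved input or resets the chain.
; Externally triggered hit checks use a looping-timer sphere sweep along the blade, or a single sphere trace for stab and kick.
; Hits on "Damagable" actors apply damage, camera shake, sound and blood, with sword hits throttled by DoOnce.
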(event Custom|SwordAttack
  ;[0.05127 0.05127 0.05127] Combo System
  ;;[0.05127 0.05127 0.05127] Sword Attack
  (if (Variables|Default|GetisAttacking)
    (Variables|Default|SetsaveAttack true)
    (else
      (Variables|Default|SetisAttacking false)
      (switch int (Variables|Default|GetattackIndex)
        (:0
          (CallFunction|Attack1))
        (:1
          (CallFunction|Attack2))
        (:2
          (CallFunction|Attack3))
        (:3
          (CallFunction|Attack4))))))

(event Custom|SwordAttackCombo
  ;[0.05127 0.05127 0.05127] Combo System
  ;;[0.05127 0.05127 0.05127] Combo
  (if (Variables|Default|GetsaveAttack)
    (Variables|Default|SetsaveAttack false)
    (switch int (Variables|Default|GetattackIndex)
      (:0
        (CallFunction|Attack1))
      (:1
        (CallFunction|Attack2))
      (:2
        (CallFunction|Attack3))
      (:3
        (CallFunction|Attack4)))
    (else
      (CallFunction|StopCombo))))

(event Custom|SphereTrace
  (bind _character_bp (Variables|Default|GetCharacter_BP))
  (bind _spheretrace (Variables|/Game/ThirdPerson/Blueprints/BP_ThirdPersonCharacter.BP_ThirdPersonCharacter_C|GetSphereTrace _character_bp))
  (bind _returnvalue (Transformation|GetWorldLocation _spheretrace))
  ;[0.05127 0.05127 0.05127] Sphere Trace for Stab & Kick
  (bind (_outhit _returnvalue_2) (Collision|SphereTraceByChannel _returnvalue _returnvalue 25.0 "TraceTypeQuery1" false 0 "None" true "(R=1.000000,G=0.000000,B=0.000000,A=1.000000)" "(R=0.000000,G=1.000000,B=0.000000,A=1.000000)" 0.2))
  (if _returnvalue_2
    (if (Actor|ActorHasTag (.HitActor (Collision|BreakHitResult _outhit)) "Damagable")
      (Game|Damage|ApplyDamage (.HitActor (Collision|BreakHitResult _outhit)) 1e+01 0 0)
      ;;[1 1 1] Camera Shake
      (Camera|PlayWorldCameraShake "/Game/Blueprints/BP_SwordHitCameraSake.BP_SwordHitCameraSake_C" (.Location (Collision|BreakHitResult _outhit)) 0.0 2e+03)
      (CallFunction|PlaySwordHitSounds)
      ;;[1 1 1] Blood Animation
      (Effects|SpawnEmitteratLocation "/Game/BloodEffectFX/Particles/Blood/P_Blood_Splat_Cone.P_Blood_Splat_Cone" (.Location (Collision|BreakHitResult _outhit)) (Math|Rotator|MakeRotfromXY (.Normal (Collision|BreakHitResult _outhit)) (.Normal (Collision|BreakHitResult _outhit))) "1.000000,1.000000,1.000000" true "AutoRelease"))))

(event Custom|PlaySwordHitSounds
  ;[0.05127 0.05127 0.05127] Play Sword Hit Sounds
  (Audio|PlaySoundatLocation "/Game/Audio/SwardHits/MS_SwordHitSounds.MS_SwordHitSounds" (Transformation|GetActorLocation (Components|GetOwner)) "0, 0, 0" 1.0 1.0 0.0 "/Game/Audio/SA_Character.SA_Character" 0 0 0))

(event Custom|StopCombo
  ;[0.05127 0.05127 0.05127] Combo System
  ;;[0.05127 0.05127 0.05127] Stop Combo / Attack
  (Variables|Default|SetisAttacking false)
  (Variables|Default|SetattackIndex 0))

(event Custom|Attack4
  ;[0.05127 0.05127 0.05127] Combo System
  ;;[0.05127 0.05127 0.05127] Attack Combo
  ;;;[0.05127 0.05127 0.05127] Attack4
  (Utilities|FlowControl|DoOnce false :!label _label
    (:Completed
      (Utilities|FlowControl|Delay 0.1)
      (Animation|Montage|PlayMontage (Variables|Default|GetcharacterMash) "/Game/Characters/Darius_Nightblade/Animations/SwordAttack/Attack3_Montage.Attack3_Montage"
        (:then
          (Variables|Default|SetattackIndex 4)
          (goto _label Reset))))))

(event Custom|Attack1
  ;[0.05127 0.05127 0.05127] Combo System
  ;;[0.05127 0.05127 0.05127] Attack Combo
  ;;;[0.05127 0.05127 0.05127] Attack1
  (Utilities|FlowControl|DoOnce false :!label _label
    (:Completed
      (Utilities|FlowControl|Delay 0.1)
      (Animation|Montage|PlayMontage (Variables|Default|GetcharacterMash) "/Game/Characters/Darius_Nightblade/Animations/SwordAttack/Attack1_Montage.Attack1_Montage"
        (:then
          (Variables|Default|SetattackIndex 1)
          (goto _label Reset))))))

(event Custom|StartSwordTrace
  ;[0.05127 0.05127 0.05127] Sword Trace
  (bind _returnvalue (Utilities|Time|SetTimerbyEvent (delegate Custom|SwordTraceLoop) 0.1 true))
  (Variables|Default|SetswordTrace _returnvalue))

(event Custom|Attack2
  ;[0.05127 0.05127 0.05127] Combo System
  ;;[0.05127 0.05127 0.05127] Attack Combo
  ;;;[0.05127 0.05127 0.05127] Attack2
  (Utilities|FlowControl|DoOnce false :!label _label
    (:Completed
      (Utilities|FlowControl|Delay 0.1)
      (Animation|Montage|PlayMontage (Variables|Default|GetcharacterMash) "/Game/Characters/Darius_Nightblade/Animations/SwordAttack/Attack2_Montage.Attack2_Montage"
        (:then
          (Variables|Default|SetattackIndex 2)
          (goto _label Reset))))))

(event Custom|SwordTraceLoop
  ;[0.05127 0.05127 0.05127] Sword Trace
  (bind (_outhit _returnvalue) (Collision|SphereTraceByChannel (Transformation|GetWorldLocation (Variables|/Game/ThirdPerson/Blueprints/BP_ThirdPersonCharacter.BP_ThirdPersonCharacter_C|GetSwordTopPoint (Variables|Default|GetCharacter_BP))) (Transformation|GetWorldLocation (Variables|/Game/ThirdPerson/Blueprints/BP_ThirdPersonCharacter.BP_ThirdPersonCharacter_C|GetSwordButtomPoint (Variables|Default|GetCharacter_BP))) 25.0 "TraceTypeQuery1" false 0 "None" true "(R=1.000000,G=0.000000,B=0.000000,A=1.000000)" "(R=0.000000,G=1.000000,B=0.000000,A=1.000000)" 0.2))
  (if _returnvalue
    (if (Actor|ActorHasTag (.HitActor (Collision|BreakHitResult _outhit)) "Damagable")
      (Utilities|FlowControl|DoOnce false :!label _label
        (:Completed
          (Game|Damage|ApplyDamage (.HitActor (Collision|BreakHitResult _outhit)) 1e+01 0 0)
          ;;[1 1 1] Camera Shake
          (Camera|PlayWorldCameraShake "/Game/Blueprints/BP_SwordHitCameraSake.BP_SwordHitCameraSake_C" (.Location (Collision|BreakHitResult _outhit)) 0.0 2e+03)
          (CallFunction|PlaySwordHitSounds)
          ;;[1 1 1] Blood Animation
          (Effects|SpawnEmitteratLocation "/Game/BloodEffectFX/Particles/Blood/P_Blood_Splat_Cone.P_Blood_Splat_Cone" (.Location (Collision|BreakHitResult _outhit)) "0.400000,0.400000,0.400000" "1.000000,1.000000,1.000000" true "AutoRelease")
          (Utilities|FlowControl|Delay 0.5)
          (goto _label Reset))))))

(event Custom|Attack3
  ;[0.05127 0.05127 0.05127] Combo System
  ;;[0.05127 0.05127 0.05127] Attack Combo
  ;;;[0.05127 0.05127 0.05127] Attack3
  (Utilities|FlowControl|DoOnce false :!label _label
    (:Completed
      (Utilities|FlowControl|Delay 0.1)
      (Animation|Montage|PlayMontage (Variables|Default|GetcharacterMash) "/Game/Characters/Darius_Nightblade/Animations/SwordAttack/Kick_Montage.Kick_Montage"
        (:then
          (Variables|Default|SetattackIndex 3)
          (goto _label Reset))))))

(event Custom|StopSwordTrace
  ;[0.05127 0.05127 0.05127] Sword Trace
  (Utilities|Time|ClearandInvalidateTimerbyHandle (Variables|Default|GetswordTrace)))

(event Input|EnhancedActionEvents|EnhancedInputActionIA_Attack
  (params (ActionValue :type Boolean) (ElapsedSeconds :type Float%20%28double-precision%29) (TriggeredSeconds :type Float%20%28double-precision%29) (InputAction :type Input%20Action%20Object%20Reference :default "/Game/ThirdPerson/Input/Actions/IA_Attack.IA_Attack"))
  ;[0.05127 0.05127 0.05127] Combo System
  ;;[0.05127 0.05127 0.05127] Attack Input
  (:Started
    (if (Variables|Default|GetcanAttack)
      (CallFunction|SwordAttack))))

(event EventBeginPlay
  (bind _asbp_third_person_character (Utilities|Casting|CastToBP_ThirdPersonCharacter (Components|GetOwner)))
  (Variables|Default|SetCharacter_BP _asbp_third_person_character)
  (Variables|Default|SetcharacterMash (Variables|/Script/Engine.Character|GetMesh _asbp_third_person_character)))